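; Player character for the basic graphics settings project, with mouse look and yaw-relative movement.
; On BeginPlay it creates a WBP_Graphics widget, without displaying it, to load saved graphics settings.
; Pressing M pauses the game, shows the mouse cursor and adds a newly created WBP_Graphics menu to the viewport.
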(event EventBeginPlay
  ;[1 1 1] Load Graphic Settings
  (bind _returnvalue (UserInterface|CreateWidget "/Game/BasicGraphicsSetting/UI/WBP_Graphics.WBP_Graphics_C"))
  (Default|LoadGraphics _returnvalue))

(event Input|AxisEvents|InputAxisTurn
  (params (AxisValue :type Float%20%28single-precision%29))
  ;[1 1 1] Mouse Control
  (Pawn|Input|AddControllerYawInput AxisValue))

(event Input|AxisEvents|InputAxisLookUp
  (params (AxisValue :type Float%20%28single-precision%29))
  ;[1 1 1] Mouse Control
  (Pawn|Input|AddControllerPitchInput AxisValue))

(event Input|AxisEvents|InputAxisForward
  (params (AxisValue :type Float%20%28single-precision%29))
  ;[1 1 1] Movement Control
  (Pawn|Input|AddMovementInput (Math|Vector|GetForwardVector (Math|Rotator|MakeRotator 0.0 0.0 (.yaw (Pawn|GetControlRotation :!class /Script/Engine.Pawn)))) AxisValue false))

(event Input|AxisEvents|InputAxisRightAndLeft
  (params (AxisValue :type Float%20%28single-precision%29))
  ;[1 1 1] Movement Control
  (Pawn|Input|AddMovementInput (Math|Vector|GetRightVector (Math|Rotator|MakeRotator 0.0 0.0 (.yaw (Pawn|GetControlRotation :!class /Script/Engine.Pawn)))) AxisValue false))

(event Input|KeyboardEvents|M
  (params (Key :type Key%20Structure :default "None"))
  ;[1 1 1] Open Menu
  (:Pressed
    (Game|SetGamePaused true)
    (Variables|/Script/Engine.PlayerController|SetbShowMouseCursor (Game|GetPlayerController 0) true)
    (bind _returnvalue (UserInterface|CreateWidget "/Game/BasicGraphicsSetting/UI/WBP_Graphics.WBP_Graphics_C"))
    (UserInterface|Viewport|AddtoViewport _returnvalue 0)))

(fn ConstructionScript)