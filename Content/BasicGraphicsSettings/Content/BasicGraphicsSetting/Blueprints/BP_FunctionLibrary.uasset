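; Blueprint function library for a graphics settings menu, driving GameUserSettings.
; GetAllResolutionsFromYourScreen fills a combo box with the supported fullscreen resolutions as "WxH" strings.
; SetGraphics switches on option type to set resolution, shadows, antialiasing, display mode or a bundled quality tier, applies the change, and returns display text for non-resolution options.
; Resolution changes also force VSync and full render scale, while SetTextures derives texture quality from screen width.
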(fn GetAllResolutionsfromYourScreen
  (params (_ComboBox :type Combo%20Box%20String%20Object%20Reference))
  (Utilities|FlowControl|DoOnce false
    (:Completed
      (bind _resolutions (Class|KismetSystemLibrary|GetSupportedFullscreenResolutions))
      (for _array_element _resolutions
        (Class|ComboBoxString|AddOption _ComboBox (Utilities|String|Append (Utilities|String|ToString(Integer) (.X (Utilities|Struct|BreakIntPoint _array_element))) "x" (Utilities|String|ToString(Integer) (.Y (Utilities|Struct|BreakIntPoint _array_element)))))))))

(fn SetGraphics
  (params (Options :type E_Graphics%20Enum :default "NewEnumerator5") (NumberOptions :type Integer) (Resolutions :type String))
  (bind (_lefts _rights) (Utilities|String|Split Resolutions "x"))
  (switch Utilities|FlowControl|Switch|SwitchonE_Graphics Options
    (:NewEnumerator5
      (bind _returnvalue (Settings|GetGameUserSettings))
      (Class|GameUserSettings|SetScreenResolution _returnvalue (Utilities|Struct|MakeIntPoint (Math|Conversions|ToInteger(Byte) _lefts) (Math|Conversions|ToInteger(Byte) _rights)))
      (Class|GameUserSettings|SetVSyncEnabled _returnvalue true)
      (Class|GameUserSettings|SetResolutionScaleValueEx _returnvalue 1e+02)
      (CallFunction|SetTextures _lefts)
      (Class|GameUserSettings|ApplySettings _returnvalue false))
    (:NewEnumerator1
      (switch int NumberOptions
        (:0
          (bind _returnvalue_2 (Settings|GetGameUserSettings))
          (Class|GameUserSettings|SetShadowQuality _returnvalue_2)
          (LocalVariables|SetText "NO"))
        (:1
          (bind _returnvalue_3 (Settings|GetGameUserSettings))
          (Class|GameUserSettings|SetShadowQuality _returnvalue_3 4)
          (LocalVariables|SetText "YES")))
      (bind _returnvalue_4 (Settings|GetGameUserSettings :!label _label))
      (Class|GameUserSettings|ApplySettings _returnvalue_4 false)
      (return (LocalVariables|GetText)))
    (:NewEnumerator2
      (switch int NumberOptions
        (:0
          (bind _returnvalue_5 (Settings|GetGameUserSettings))
          (Class|GameUserSettings|SetAntiAliasingQuality _returnvalue_5)
          (LocalVariables|SetText "NO")
          (goto _label))
        (:1
          (bind _returnvalue_6 (Settings|GetGameUserSettings))
          (Class|GameUserSettings|SetAntiAliasingQuality _returnvalue_6 4)
          (LocalVariables|SetText "YES")
          (goto _label))))
    (:NewEnumerator3
      (switch int NumberOptions
        (:0
          (bind _returnvalue_7 (Settings|GetGameUserSettings))
          (Class|GameUserSettings|SetFullscreenMode _returnvalue_7 "Windowed")
          (LocalVariables|SetText "WINDOWED")
          (goto _label))
        (:1
          (bind _returnvalue_8 (Settings|GetGameUserSettings))
          (Class|GameUserSettings|SetFullscreenMode _returnvalue_8 "Fullscreen")
          (LocalVariables|SetText "FULLSCREEN")
          (goto _label))))
    (:NewEnumerator4
      (switch int NumberOptions
        (:0
          (bind _returnvalue_9 (Settings|GetGameUserSettings))
          (Class|GameUserSettings|SetPostProcessingQuality _returnvalue_9)
          (Class|GameUserSettings|SetViewDistanceQuality _returnvalue_9)
          (Class|GameUserSettings|SetVisualEffectQuality _returnvalue_9)
          (Class|GameUserSettings|SetFoliageQuality _returnvalue_9)
          (LocalVariables|SetText "LOW")
          (goto _label))
        (:1
          (bind _returnvalue_10 (Settings|GetGameUserSettings))
          (Class|GameUserSettings|SetPostProcessingQuality _returnvalue_10 1)
          (Class|GameUserSettings|SetViewDistanceQuality _returnvalue_10 1)
          (Class|GameUserSettings|SetVisualEffectQuality _returnvalue_10 1)
          (Class|GameUserSettings|SetFoliageQuality _returnvalue_10 1)
          (LocalVariables|SetText "MEDIUM")
          (goto _label))
        (:2
          (bind _returnvalue_11 (Settings|GetGameUserSettings))
          (Class|GameUserSettings|SetPostProcessingQuality _returnvalue_11 2)
          (Class|GameUserSettings|SetViewDistanceQuality _returnvalue_11 2)
          (Class|GameUserSettings|SetVisualEffectQuality _returnvalue_11 2)
          (Class|GameUserSettings|SetFoliageQuality _returnvalue_11 2)
          (LocalVariables|SetText "HIGH")
          (goto _label))
        (:3
          (bind _returnvalue_12 (Settings|GetGameUserSettings))
          (Class|GameUserSettings|SetPostProcessingQuality _returnvalue_12 3)
          (Class|GameUserSettings|SetViewDistanceQuality _returnvalue_12 3)
          (Class|GameUserSettings|SetVisualEffectQuality _returnvalue_12 3)
          (Class|GameUserSettings|SetFoliageQuality _returnvalue_12 3)
          (LocalVariables|SetText "ULTRA")
          (goto _label))
        (:4
          (bind _returnvalue_13 (Settings|GetGameUserSettings))
          (Class|GameUserSettings|SetPostProcessingQuality _returnvalue_13 4)
          (Class|GameUserSettings|SetViewDistanceQuality _returnvalue_13 4)
          (Class|GameUserSettings|SetVisualEffectQuality _returnvalue_13 4)
          (Class|GameUserSettings|SetFoliageQuality _returnvalue_13 4)
          (LocalVariables|SetText "HYPER")
          (goto _label))))))

(fn SetTextures
  (params (ResolutionX :type String))
  (bind _returnvalue (Math|Conversions|ToInteger(Byte) ResolutionX))
  (if (< (Math|Conversions|ToInteger(Byte) ResolutionX) 1280)
    (bind _returnvalue_2 (Settings|GetGameUserSettings))
    (Class|GameUserSettings|SetTextureQuality _returnvalue_2 1)
    (elif (and (>= _returnvalue 1280) (< _returnvalue 1920))
      (bind _returnvalue_3 (Settings|GetGameUserSettings))
      (Class|GameUserSettings|SetTextureQuality _returnvalue_3 3)
      (elif (>= (Math|Conversions|ToInteger(Byte) ResolutionX) 1920)
        (bind _returnvalue_4 (Settings|GetGameUserSettings))
        (Class|GameUserSettings|SetTextureQuality _returnvalue_4 4)))))