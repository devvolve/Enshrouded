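; Inventory component that holds a fixed-size array of item slots, set up on BeginPlay, with server events for adding and transferring items.
; Adding fills matching stacks using the stack size from each item's data asset, then splits the remainder across empty slots.
; Transfers between indices or components place, stack or swap items, using each slot's stored inventory reference to update the source.
; Slot writes broadcast an OnSlotChanged notification.
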(event Custom|SetupSlotServer
  (params (SlotAmount :type Integer))
  ;[1 1 1] Setup inventory slots on server
  (bind _output_get (Variables|Default|SetSlotAmount SlotAmount))
  (for _index (range 0 (- _output_get 1))
    (Utilities|Array|Add (Variables|Default|GetItemSlots) (Utilities|Struct|MakeS_InventorySlots _index self))))

(event Custom|AddItemServer
  (params (ItemsToAdd :type S%20Inventory%20Slots%20Structure))
  (CallFunction|AddItem ItemsToAdd))

(event Custom|TransferItemServer
  (params (ToInventoryComponent :type BPC%20Inventory%20Object%20Reference) (FromIndex :type Integer) (ToIndex :type Integer))
  (Transfer|TransferItem ToInventoryComponent FromIndex ToIndex))

(event EventBeginPlay
  (CallFunction|SetupSlotServer (Variables|Default|GetSlotAmount)))

(fn AddItem
  (params (ItemsToAdd :type S%20Inventory%20Slots%20Structure))
  (bind _output_get (LocalVariables|SetCurrentItemToAdd ItemsToAdd))
  (bind _returnvalue (Utilities|LoadAssetBlocking (Utilities|Struct|BreakS_InventorySlots _output_get)))
  (bind (_isstackable _stacksize) (Class|BPIAssets|IsItemStackable(Message) _returnvalue))
  (LocalVariables|SetItemStackSize _stacksize)
  (if _isstackable
    ;[1 1 1] check slots in inventory with same item & item in stackable
    (for _array_element (Variables|Default|GetItemSlots)
      (bind _output_get_2 (LocalVariables|SetTargetSlot _array_element))
      (if (.Result (CallFunction|IsStackableandHaveSpace _output_get_2 (LocalVariables|GetCurrentItemToAdd)))
        (bind _output_get_3 (LocalVariables|SetNewQuantityFromTargetSLot (+ (Utilities|Struct|BreakS_InventorySlots _array_element) (Utilities|Struct|BreakS_InventorySlots (LocalVariables|GetCurrentItemToAdd)))))
        (if (> _output_get_3 (LocalVariables|GetItemStackSize))
          (Setter/Getter|SetQuantityatSlot (LocalVariables|GetTargetSlot) (LocalVariables|GetItemStackSize))
          (Utilities|Struct|SetmembersinS_InventorySlots (LocalVariables|GetCurrentItemToAdd) (- (LocalVariables|GetNewQuantityFromTargetSLot) (LocalVariables|GetItemStackSize)))
          (else
            (Setter/Getter|SetQuantityatSlot (LocalVariables|GetTargetSlot) (LocalVariables|GetNewQuantityFromTargetSLot))
            (return true))))))
  ;[1 1 1] Add Item To empty slots
  (bind (_result _slot) (Search|FindEmptySlot :!label _label))
  (if _result
    (LocalVariables|SetTargetSlot _slot)
    (if (<= (.Quantity (Utilities|Struct|BreakS_InventorySlots (LocalVariables|GetCurrentItemToAdd))) (LocalVariables|GetItemStackSize))
      (Setter/Getter|SetItem (LocalVariables|GetTargetSlot) (LocalVariables|GetCurrentItemToAdd))
      (return true)
      (else
        (bind _output_get_4 (LocalVariables|SetTemporaryCacheItemToAdd (LocalVariables|GetCurrentItemToAdd)))
        (bind _structout (Utilities|Struct|SetmembersinS_InventorySlots _output_get_4 (LocalVariables|GetItemStackSize)))
        (Setter/Getter|SetItem (LocalVariables|GetTargetSlot) _structout)
        (Utilities|Struct|SetmembersinS_InventorySlots (LocalVariables|GetCurrentItemToAdd) (- (Utilities|Struct|BreakS_InventorySlots (LocalVariables|GetCurrentItemToAdd)) (LocalVariables|GetItemStackSize)))
        (goto _label)))
    (else
      (Development|PrintString "Inventory is FULL")
      (return false))))

(fn FindEmptySlot
  (for _array_element (Variables|Default|GetItemSlots)
    (if (CallFunction|IsSlotEmpty _array_element)
      (return true _array_element))))

(fn SetItem
  (params (TargetSlot :type S%20Inventory%20Slots%20Structure) (Item :type S%20Inventory%20Slots%20Structure))
  (bind _slotindex (Utilities|Struct|BreakS_InventorySlots TargetSlot))
  (Utilities|Array|SetArrayElem (Variables|Default|GetItemSlots) _slotindex Item)
  (bind _structout (Utilities|Struct|SetmembersinS_InventorySlots (Utilities|Array|Get(acopy) (Variables|Default|GetItemSlots) _slotindex) _slotindex self))
  (Default|CallOnSlotChanged _structout))

(fn SetQuantityatSlot
  (params (TargetSlot :type S%20Inventory%20Slots%20Structure) (Quantity :type Integer))
  (bind _structout (Utilities|Struct|SetmembersinS_InventorySlots (Utilities|Array|Get(acopy) (Variables|Default|GetItemSlots) (Utilities|Struct|BreakS_InventorySlots TargetSlot)) Quantity))
  (Default|CallOnSlotChanged _structout)
  (return _structout))

(fn TransferItem
  (params (ToInventoryComponent :type BPC%20Inventory%20Object%20Reference) (FromIndex :type Integer) (ToIndex :type Integer))
  (if (and (== self ToInventoryComponent) (== FromIndex ToIndex))
    (Development|PrintString "Error: Same container & same slot")
    (return false)
    (elif (Math|Boolean|ANDBoolean (Utilities|IsValid ToInventoryComponent) (.IsValid (Setter/Getter|GetSlotIndex FromIndex)) (or (.IsValid (Setter/Getter|GetSlotIndex ToInventoryComponent ToIndex)) (== ToIndex -1)))
      (if (== ToIndex -1)
        (Development|PrintString "Target slot index is not specified")
        (else
          (bind (_successfully _areallitemsadded) (CallFunction|AddItemtoIndex ToInventoryComponent ToIndex (.Slot (Setter/Getter|GetSlotIndex FromIndex))))
          (if _successfully
            (if _areallitemsadded
              (bind _successfully_2 (CallFunction|RemoveItemfromIndex FromIndex))
              (return _successfully_2)
              (else
                (return true)))
            (else
              (return false)))))
      (else
        (return false)))))

(fn GetSlotIndex
  (params (Index :type Integer))
  (if (Utilities|Array|IsValidIndex (Variables|Default|GetItemSlots) Index)
    (return true (Utilities|Array|Get(acopy) (Variables|Default|GetItemSlots) Index))
    (else
      (return false ""))))

(fn AddItemtoIndex
  (params (TargetIndex :type Integer) (ItemSlotToAdd :type S%20Inventory%20Slots%20Structure))
  (bind (_isvalid _slot) (Setter/Getter|GetSlotIndex TargetIndex))
  (if _isvalid
    (if (CallFunction|IsSlotEmpty _slot)
      (Setter/Getter|SetItem _slot ItemSlotToAdd)
      (return true true)
      (else
        (bind _areallitemsadded (Transfer|StackItemonTransfer _slot ItemSlotToAdd))
        (return true _areallitemsadded)))
    (else
      (return false false))))

(fn StackItemonTransfer
  (params (TargetSlot :type S%20Inventory%20Slots%20Structure) (FromSlot :type S%20Inventory%20Slots%20Structure))
  (bind (_result _itemstacksize) (CallFunction|IsStackableandHaveSpace TargetSlot FromSlot))
  (if _result
    (LocalVariables|SetItemStackSize _itemstacksize)
    (bind _output_get (LocalVariables|SetNewQuantityFromTargetSLot (+ (Utilities|Struct|BreakS_InventorySlots TargetSlot) (Utilities|Struct|BreakS_InventorySlots FromSlot))))
    (if (> _output_get (LocalVariables|GetItemStackSize))
      (Setter/Getter|SetQuantityatSlot TargetSlot (LocalVariables|GetItemStackSize))
      (Setter/Getter|SetQuantityatSlot (Utilities|Struct|BreakS_InventorySlots FromSlot) FromSlot (- (LocalVariables|GetNewQuantityFromTargetSLot) (LocalVariables|GetItemStackSize)))
      (return false)
      (else
        (Setter/Getter|SetQuantityatSlot TargetSlot (LocalVariables|GetNewQuantityFromTargetSLot))
        (return true)))
    (else
      ;[1 1 1] swap index
      (Transfer|SwapIndexes TargetSlot FromSlot)
      (return false))))

(fn RemoveItemfromIndex
  (params (Index :type Integer))
  (bind (_isvalid _slot) (Setter/Getter|GetSlotIndex Index))
  (if _isvalid
    (Setter/Getter|SetItem _slot (Utilities|Struct|MakeS_InventorySlots))
    (return true)
    (else
      (return false))))

(fn SwapIndexes
  (params (Slot :type S%20Inventory%20Slots%20Structure) (Swap :type S%20Inventory%20Slots%20Structure))
  (Setter/Getter|SetItem Slot Swap)
  (Setter/Getter|SetItem (Utilities|Struct|BreakS_InventorySlots Swap) Swap Slot))